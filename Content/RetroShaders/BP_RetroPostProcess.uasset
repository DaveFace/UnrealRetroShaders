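; Retro post-process actor that applies a pixelated look with colour banding and dithering, toggled at runtime with the L key.
; The construction script creates a dynamic PPI_RetroLook material, assigns it as a post-process blendable and sets its parameters.
; BeginPlay sets nearest-neighbour upscaling for sharp pixels and ticks only when UseDownsample is on.
; A Delay-throttled Tick polls viewport size, recalculating screen percentage from DownsampleResolution when it changes.
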(event EventBeginPlay
  (Input|EnableInput (Game|GetPlayerController 0))
  ;[0 0.1193 1] These would be better placed in your 'device profiles' settings
  (Development|ExecuteConsoleCommand "r.upscale.quality 0" 0) ; This sets the upscale interpolation to point / nearest neighbor\nso that when we downsample at runtime, the result is nice\nsharp pixels instead of a blurry mess
  (Development|ExecuteConsoleCommand "sg.resolutionquality 100" 0)
  (Actor|Tick|SetActorTickEnabled (Variables|Configuration|GetbUseDownsample)))

(event EventTick
  (params (DeltaSeconds :type Float%20%28single-precision%29))
  (Utilities|FlowControl|Delay 0.5)
  ;[0 1 0.364] Downsample functions; only processed at runtime
  (bind _returnvalue (CallFunction|CheckforResolutionChange))
  (if _returnvalue
    (CallFunction|SetDownsampleRes)))

(event Input|KeyboardEvents|L
  (params (Key :type Key%20Structure :default "None"))
  ;[1 0 0.4074] Enable / Disable Debug
  (:Pressed
    (bind _output_get (Variables|/Script/Engine.PostProcessComponent|SetbEnabled (Variables|Default|GetPostProcess) (not (Variables|Configuration|GetbEnabled))))
    (bind _output_get_2 (Variables|Configuration|SetbEnabled _output_get))
    (Development|PrintString (Utilities|String|Append "Retro Post Process turned " (select _output_get_2 "ON" "OFF")))))

(fn ConstructionScript
  (Variables|/Script/Engine.PostProcessComponent|SetbEnabled (Variables|Default|GetPostProcess) (Variables|Configuration|GetbEnabled))
  (Utilities|FlowControl|Sequence
    (:then_0
      ;[0 0.6815 1] Create the material instance and apply it to post process
      (bind _returnvalue (Rendering|Material|CreateDynamicMaterialInstance "/Game/RetroShaders/PostProcess/PPI_RetroLook.PPI_RetroLook" "None" :!class /Script/Engine.KismetMaterialLibrary))
      (bind _output_get (Variables|Internal|SetRetroLookRef _returnvalue))
      (Variables|/Script/Engine.PostProcessComponent|SetSettings (Variables|Default|GetPostProcess) (Utilities|Struct|MakePostProcessSettings (Utilities|Struct|MakeWeightedBlendables (Utilities|Array|MakeArray (Utilities|Struct|MakeWeightedBlendable 1.0 _output_get))))))
    (:then_1
      ;[1 0 0.1981] Set parameters
      (Rendering|Material|SetScalarParameterValue (Variables|Internal|GetRetroLookRef) "ColourBanding" (Variables|Configuration|GetColourBanding) :!class /Script/Engine.MaterialInstanceDynamic)
      (Rendering|Material|SetScalarParameterValue (Variables|Internal|GetRetroLookRef) "VerticalResolution" (Variables|Configuration|GetVerticalResolution) :!class /Script/Engine.MaterialInstanceDynamic)
      (Rendering|Material|SetScalarParameterValue (Variables|Internal|GetRetroLookRef) "DitherLerp" (Variables|Configuration|GetDitheringLerp) :!class /Script/Engine.MaterialInstanceDynamic))))

(fn CheckforResolutionChange
  (LocalVariables|SetbIsResSame (Math|Vector|Equal(Vector) (Variables|Internal|GetLastResolutionSize) (Viewport|GetViewportSize) 0.0001))
  (Variables|Internal|SetLastResolutionSize (Viewport|GetViewportSize))
  (return (not (LocalVariables|GetbIsResSame))))

(fn SetDownsampleRes
  (Development|ExecuteConsoleCommand (Utilities|String|Append "r.ScreenPercentage " (Utilities|String|ToString(Float) (* (Math|Float|Clamp(Float) (/ (Variables|Configuration|GetDownsampleResolution) (.Y (Math|Vector2D|BreakVector2D (Viewport|GetViewportSize))))) 1e+02))) 0)
  (return))