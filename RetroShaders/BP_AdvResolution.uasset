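; BP_AdvResolution is an actor that applies a retro post-process look with adjustable low resolution, colour banding and dithering.
; On BeginPlay it adds a dynamic PP_RetroLook material to RetroPostProcess and sets upscale and resolution-quality console variables.
; Tick watches for viewport size changes, then derives r.ScreenPercentage from RenderResolution and sets the material's PixelFactor from FinalResolution relative to that downsampled height.
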(event EventBeginPlay
  (Resolution|CreatePostProcess)
  ;[1 1 1] These would be better placed in your 'device profiles' settings
  (Development|ExecuteConsoleCommand "r.upscale.quality 0" 0)
  (Development|ExecuteConsoleCommand "sg.resolutionquality 100" 0))

(event EventTick
  (params (DeltaSeconds :type Float%20%28single-precision%29))
  (bind _changed (Resolution|CheckResChange))
  (if _changed
    (Resolution|CalculateDownsampleRes)))

(fn ConstructionScript)

(fn CalculateDownsampleRes
  (bind _returnvalue (Viewport|GetViewportSize))
  (bind _renderresolution (Variables|GlobalSettings|GetRenderResolution))
  (bind _y (Math|Vector2D|BreakVector2D _returnvalue))
  (bind _returnvalue_2 (/ _renderresolution _y))
  (bind _returnvalue_3 (Math|Float|Clamp(Float) _returnvalue_2))
  (Development|ExecuteConsoleCommand (Utilities|String|Append "r.ScreenPercentage " (Utilities|String|ToString(Float) (* _returnvalue_3 1e+02))) 0)
  (Rendering|Material|SetScalarParameterValue (Variables|Internal|GetPPRetroInstance) "PixelFactor" (/ (Variables|GlobalSettings|GetFinalResolution) (* _returnvalue_3 _y)) :!class /Script/Engine.MaterialInstanceDynamic))

(fn CheckResChange
  (bind _returnvalue (Viewport|GetViewportSize))
  (LocalVariables|SetIsResSame (Math|Vector|Equal(Vector) (Variables|Internal|GetLastResolutionSize) _returnvalue 0.0001))
  (Variables|Internal|SetLastResolutionSize _returnvalue)
  (return (not (LocalVariables|GetIsResSame))))

(fn CreatePostProcess
  ;[1 0 0.3547] Create material instance and add it to post process
  (bind _returnvalue (Rendering|Material|CreateDynamicMaterialInstance "/Game/RetroShaders/PostProcess/PP_RetroLook.PP_RetroLook" "None" :!class /Script/Engine.KismetMaterialLibrary))
  (bind _output_get (Variables|Internal|SetPPRetroInstance _returnvalue))
  (Variables|/Script/Engine.PostProcessComponent|SetSettings (Variables|Default|GetRetroPostProcess) (Utilities|Struct|MakePostProcessSettings (Utilities|Struct|MakeWeightedBlendables (Utilities|Array|MakeArray (Utilities|Struct|MakeWeightedBlendable 1.0 _output_get)))))
  ;[0.3422 1 0.2124] Set Parameters
  (Rendering|Material|SetScalarParameterValue (Variables|Internal|GetPPRetroInstance) "ColourBanding" (Variables|LevelSettings|GetColourBanding) :!class /Script/Engine.MaterialInstanceDynamic)
  (Rendering|Material|SetScalarParameterValue (Variables|Internal|GetPPRetroInstance) "DitherBlending" (Variables|LevelSettings|GetDitherBlending) :!class /Script/Engine.MaterialInstanceDynamic)
  (Rendering|Material|SetScalarParameterValue (Variables|Internal|GetPPRetroInstance) "DitherBlackLevels" (Variables|LevelSettings|GetDitherBlackLevel) :!class /Script/Engine.MaterialInstanceDynamic)
  (Rendering|Material|SetScalarParameterValue (Variables|Internal|GetPPRetroInstance) "DitherMaskPower" (Variables|LevelSettings|GetDitherBlackLevel) :!class /Script/Engine.MaterialInstanceDynamic))